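; BP_Trigger is a trigger actor that changes its light color and counts how many times its box is entered.
; Box begin and end overlap set IsActorEntered, then share one branch that turns the PointLight purple while entered and red after exit.
; The entered branch also increments Score and prints it on screen.
; Any overlap counts, with no filter on the other actor.
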(event OnComponentBeginOverlap(Box)
  (params (OverlappedComponent :type Primitive%20Component%20Object%20Reference) (OtherActor :type Actor%20Object%20Reference) (OtherComp :type Primitive%20Component%20Object%20Reference) (OtherBodyIndex :type Integer) (bFromSweep :type Boolean) (SweepResult :type Hit%20Result%20Structure%20%28by%20ref%29))
  (Variables|Default|SetisActorEntered? true)
  (if (Variables|Default|GetisActorEntered?)
    (Rendering|Components|Light|SetLightColor (Variables|Default|GetPointLight) "(R=0.213362,G=0.000000,B=0.281250,A=1.000000)" true)
    (CallFunction|Score++)
    (else
      (Rendering|Components|Light|SetLightColor (Variables|Default|GetPointLight) "(R=0.843750,G=0.000000,B=0.000000,A=1.000000)" true))))

(event OnComponentEndOverlap(Box)
  (params (OverlappedComponent :type Primitive%20Component%20Object%20Reference) (OtherActor :type Actor%20Object%20Reference) (OtherComp :type Primitive%20Component%20Object%20Reference) (OtherBodyIndex :type Integer))
  (Variables|Default|SetisActorEntered? false)
  (if (Variables|Default|GetisActorEntered?)
    (Rendering|Components|Light|SetLightColor (Variables|Default|GetPointLight) "(R=0.213362,G=0.000000,B=0.281250,A=1.000000)" true)
    (CallFunction|Score++)
    (else
      (Rendering|Components|Light|SetLightColor (Variables|Default|GetPointLight) "(R=0.843750,G=0.000000,B=0.000000,A=1.000000)" true))))

(event EventBeginPlay)

(event Collision|EventActorBeginOverlap
  (params (OtherActor :type Actor%20Object%20Reference)))

(event EventTick
  (params (DeltaSeconds :type Float%20%28single-precision%29)))

(fn ConstructionScript)

(fn Score++
  (bind _result (Math|Integer|IncrementInt (Variables|Default|GetScore))
    (:%20%20
      (bind _output_get (Variables|Default|SetScore _result))
      (Development|PrintString (Utilities|String|ToString(Integer) _output_get) true true "(R=0.942708,G=0.004910,B=0.121040,A=1.000000)" 5.0))))