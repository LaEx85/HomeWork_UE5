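; BP_DataTrigger is a homework trigger actor that prints debug messages when something enters or leaves its Box.
; Begin overlap picks a random row from the DT_ItemInventory data table and prints its name, count and description.
; End overlap calls SumRandomAndCount, which prints a random integer from 1 to 5 plus a Count array element.
; The loop over Count never runs, so that element is never iterated.
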(event OnComponentBeginOverlap(Box)
  (params (OverlappedComponent :type Primitive%20Component%20Object%20Reference) (OtherActor :type Actor%20Object%20Reference) (OtherComp :type Primitive%20Component%20Object%20Reference) (OtherBodyIndex :type Integer) (bFromSweep :type Boolean) (SweepResult :type Hit%20Result%20Structure%20%28by%20ref%29))
  (bind _outrownames (DataTable|GetDataTableRowNames "/Game/HomeWork/HW3/Bluprints/Actor/DT_ItemInventory.DT_ItemInventory"))
  (bind _returnvalue (Utilities|GetDataTableRow "/Game/HomeWork/HW3/Bluprints/Actor/DT_ItemInventory.DT_ItemInventory" (.OutItem (Utilities|Array|Random _outrownames)))
    (:then
      (Development|PrintString (Utilities|String|ToString(Text) (Utilities|Text|FormatText "You got  {Name} {Count} {Description} " (Utilities|String|ToString(Name) (.Name (Utilities|Struct|BreakS_ItemInventory _returnvalue))) (.Count (Utilities|Struct|BreakS_ItemInventory _returnvalue)) (.Description (Utilities|Struct|BreakS_ItemInventory _returnvalue))))))))

(event OnComponentEndOverlap(Box)
  (params (OverlappedComponent :type Primitive%20Component%20Object%20Reference) (OtherActor :type Actor%20Object%20Reference) (OtherComp :type Primitive%20Component%20Object%20Reference) (OtherBodyIndex :type Integer))
  (CallFunction|SumRandomandCount))

(event EventBeginPlay)

(fn ConstructionScript)

(fn SumRandomandCount
  (Development|PrintString (Utilities|String|ToString(Text) (Utilities|Text|FormatText "Answer {Sum}" (+ (Math|Random|RandomIntegerinRange 1 5) (stale _array_element)))) true true "(R=0.019022,G=0.913043,B=0.059487,A=1.000000)" 1.0))