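; Elevator actor that toggles its mesh between two positions when something begins overlapping its trigger box.
; The overlap plays the MoveTimeElevator timeline forward or in reverse according to TargetElevator, with BlockMoving ignoring new triggers until it finishes and flips the direction.
; Each timeline update sets the mesh's relative location by a lerp between start and end points, but with a constant alpha instead of a timeline track.
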(event OnComponentBeginOverlap(Box)
  (params (OverlappedComponent :type Primitive%20Component%20Object%20Reference) (OtherActor :type Actor%20Object%20Reference) (OtherComp :type Primitive%20Component%20Object%20Reference) (OtherBodyIndex :type Integer) (bFromSweep :type Boolean) (SweepResult :type Hit%20Result%20Structure%20%28by%20ref%29))
  (if (not (Variables|Default|GetBlockMoving))
    (Variables|Default|SetBlockMoving true)
    (if (Variables|Default|GetTargetElevator)
      (Timeline|MoveTimeElevator ReverseFromEnd
        (:Update
          (Transformation|SetRelativeLocation (Variables|Default|GetStaticMesh) (Math|Vector|Lerp(Vector) (Variables|Default|GetStartingPoint) (Variables|Default|GetEndPoint) 2.0) false false))
        (:Finished
          (Variables|Default|SetTargetElevator (not (Variables|Default|GetTargetElevator)))
          (Variables|Default|SetBlockMoving false)))
      (else
        (Timeline|MoveTimeElevator PlayFromStart)))))

(event OnComponentEndOverlap(Box)
  (params (OverlappedComponent :type Primitive%20Component%20Object%20Reference) (OtherActor :type Actor%20Object%20Reference) (OtherComp :type Primitive%20Component%20Object%20Reference) (OtherBodyIndex :type Integer)))

(event EventBeginPlay
  (Variables|Default|SetStartingPoint "0.000000,0.000000,0.000000")
  (Variables|Default|SetEndPoint "0.000000,0.000000,100.000000"))

(fn ConstructionScript)