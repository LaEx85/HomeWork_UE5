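; BP_TriggerEnum is a trigger actor that demonstrates switching on a weapon type enum when something overlaps its Box.
; On each overlap, Weapon prints the name of the current weapon type through a switch on the enum.
; RandomEnum then picks a random integer, casts it to E_WeaponType and stores it, so the new value is printed on the following overlap.
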(event OnComponentBeginOverlap(Box)
  (params (OverlappedComponent :type Primitive%20Component%20Object%20Reference) (OtherActor :type Actor%20Object%20Reference) (OtherComp :type Primitive%20Component%20Object%20Reference) (OtherBodyIndex :type Integer) (bFromSweep :type Boolean) (SweepResult :type Hit%20Result%20Structure%20%28by%20ref%29))
  (CallFunction|Weapon)
  (CallFunction|RandomEnum))

(event EventBeginPlay)

(fn ConstructionScript)

(fn Weapon
  (switch Utilities|FlowControl|Switch|SwitchonE_WeaponType (Variables|Default|GetCurrentWeapontType)
    (:NewEnumerator0
      (Development|PrintString "Knife" true true "(R=1.000000,G=0.000000,B=0.428912,A=1.000000)" 5.0))
    (:NewEnumerator1
      (Development|PrintString "Pistol" true true "(R=1.000000,G=0.000000,B=0.428912,A=1.000000)" 5.0))
    (:NewEnumerator2
      (Development|PrintString "Rifle" true true "(R=1.000000,G=0.000000,B=0.428912,A=1.000000)" 5.0))
    (:NewEnumerator3
      (Development|PrintString "Sniper Rifle" true true "(R=1.000000,G=0.000000,B=0.428912,A=1.000000)" 5.0))
    (:NewEnumerator4
      (Development|PrintString "Grenade" true true "(R=1.000000,G=0.000000,B=0.428912,A=1.000000)" 5.0))))

(fn RandomEnum
  (bind _returnvalue (Math|Random|RandomIntegerinRange 0 4))
  (Variables|Default|SetCurrentWeapontType (Utilities|Enum|ByteToEnumE_WeaponType (Math|Conversions|ToByte(Integer) _returnvalue))))